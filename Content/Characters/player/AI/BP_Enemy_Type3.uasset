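; Enemy character Blueprint for the Type 3 AI enemy, implementing its death sequence.
; Die calls a server-named event that forwards to a multi-named event, following an RPC-style pattern for networked death.
; That event disables movement, enables mesh physics simulation and plays a death montage, then sets IsDead and destroys the actor after a short delay.
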(event Custom|ServerSpawnEnemy3Die
  (CallFunction|MultiSpawnEnemy3Die))

(event Custom|MultiSpawnEnemy3Die
  ;[1 1 1] Death motion
  (Pawn|Components|CharacterMovement|DisableMovement (Variables|Character|GetCharacterMovement))
  (Physics|SetSimulatePhysics (Variables|Character|GetMesh) true)
  (Animation|Montage|PlayMontage 0 (Variables|Default|GetDeathAnims)
    (:then
      (Variables|Default|SetIsDead? true)
      (Utilities|FlowControl|Delay 2.0)
      (Actor|DestroyActor))))

(event EventBeginPlay
  (|CallParentFunction) ; This node is disabled and will not be called.\nDrag off pins to build functionality.
)

(event Collision|EventActorBeginOverlap
  (params (OtherActor :type Actor%20Object%20Reference)))

(event EventTick
  (params (DeltaSeconds :type Float%20%28single-precision%29)))

(event EventDie
  (CallFunction|ServerSpawnEnemy3Die))

(fn ConstructionScript
  (|CallParentFunction))