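; BPC_Stats is a stats component that tracks health and mana for its owning actor, with a preset for boss health.
; IncreaseValue applies clamped changes to either stat and updates the progress bar handed in through setter events.
; Health reaching zero triggers DieMessage on the owner.
; A fast looping timer adds a small amount of mana while BombCast is true.
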(event Custom|Die
  (Class|BPIDamage|Die(Message) (Components|GetOwner)))

(event Custom|Set%20Mana%20ProgressBar
  (params (Mana%20Progress%20Bar :type Progress%20Bar%20Object%20Reference))
  (Variables|Default|SetMana%20Progress%20Bar Mana%20Progress%20Bar))

(event Custom|Set%20Health%20Progress%20Bar
  (params (Health%20Progress%20Bar :type Progress%20Bar%20Object%20Reference))
  (Variables|Default|SetHealth%20Progress%20Bar Health%20Progress%20Bar))

(event Custom|using%20Mana
  (if (Variables|Default|GetBombCast?)
    (CallFunction|IncreaseValue "NewEnumerator1" 0.1)))

(event EventBeginPlay
  (Utilities|Time|SetTimerbyEvent (delegate Custom|using%20Mana) 0.01 true))

(fn IncreaseValue
  (params (Stats :type E_Stats%20Enum :default "E_Stats_MAX") (Value :type Float%20%28double-precision%29))
  (switch Utilities|FlowControl|Switch|SwitchonE_Stats Stats
    (:NewEnumerator0
      (Variables|Default|Sethealth (Math|Float|Clamp(Float) (+ (Variables|Default|Gethealth) Value) 0.0 (Variables|Default|GetMaxHealth)))
      (Utilities|FlowControl|Sequence
        (:then_0
          (if (<= (Variables|Default|Gethealth) 0.0)
            (CallFunction|Die)))
        (:then_1
          (bind _health_progress_bar (Variables|Default|GetHealth%20Progress%20Bar)
            (:then
              (Progress|SetPercent _health_progress_bar (/ (Variables|Default|Gethealth) (Variables|Default|GetMaxHealth))))
            (:else)))))
    (:NewEnumerator1
      (Variables|Default|SetMana (Math|Float|Clamp(Float) (+ (Variables|Default|GetMana) Value) 0.0 (Variables|Default|GetmaxMana)))
      (bind _mana_progress_bar (Variables|Default|GetMana%20Progress%20Bar)
        (:then
          (Progress|SetPercent _mana_progress_bar (/ (Variables|Default|GetMana) (Variables|Default|GetmaxMana))))
        (:else)))))

(fn BossHealth
  (Variables|Default|SetMaxHealth 5e+02)
  (Variables|Default|Sethealth 5e+02))